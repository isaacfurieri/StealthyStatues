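; Museum guard AI character that catches the player on overlap unless they are disguised as a statue.
; Each Tick spins its five question-mark indicators and scans the Guard component's overlaps for a component named "Player".
; A statue player hides the alert sprite and shows the question marks.
; Otherwise the level fails: Level_1_M4 shows a paused failure dialog, while other levels open the LevelFailed map.
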(event Custom|ShowConfused
  (params (Confused :type Boolean))
  (Rendering|SetVisibility (Variables|Default|GetQuestionMark) Confused false))

(event EventTick
  (params (DeltaSeconds :type Float%20%28single-precision%29))
  (Utilities|FlowControl|Sequence
    (:then_0
      (Transformation|AddLocalRotation (Variables|Default|GetQuestionMark) "0.000000,1.000000,0.000000" false false))
    (:then_1
      (for _array_element (Class|PrimitiveComponent|GetOverlappingComponents (Variables|Default|GetGuard))
        (if (Utilities|Enum|Equal(Enum) "Player" (Utilities|GetObjectName _array_element))
          (bind _asbp_top_down_character (Utilities|Casting|CastToBP_TopDownCharacter (Game|GetPlayerCharacter 0)))
          (if (Variables|/Game/TopDown/Blueprints/BP_TopDownCharacter.BP_TopDownCharacter_C|GetIsStatue _asbp_top_down_character)
            (CallFunction|ToggleAlertSprite false)
            (CallFunction|ShowConfused true)
            (else
              (bind _returnvalue (Game|GetCurrentLevelName true))
              (if (Utilities|Enum|Equal(Enum) _returnvalue "Level_1_M4")
                (bind _returnvalue_2 (UserInterface|CreateWidget "/Game/UI/Level1Tutorial/WBP_Level1FailedDialog.WBP_Level1FailedDialog_C"))
                (UserInterface|Viewport|AddtoViewport _returnvalue_2 0)
                (Game|SetGamePaused true)
                (else
                  (Game|OpenLevel(byObjectReference) "/Game/UI/LevelFailed/LevelFailed.LevelFailed"))))))))))

(fn ConstructionScript)

(fn ToggleAlertSprite
  (params (IsVisible :type Boolean))
  (Rendering|SetVisibility (Variables|Default|GetAlert) IsVisible false)
  (Rendering|SetVisibility (Variables|Default|GetAlertDot) IsVisible false))
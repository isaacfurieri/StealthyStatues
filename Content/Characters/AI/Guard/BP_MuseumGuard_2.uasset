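; BP_MuseumGuard_2 is a museum guard AI character Blueprint with a toggleable alert indicator.
; ToggleAlertSprite shows or hides the Alert and AlertDot components together.
; The event graph has no active logic, only an unconnected capsule-overlap loop that would open LevelFailed whether or not the component's name is "Guard".
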(event EventBeginPlay)

(event Collision|EventActorBeginOverlap
  (params (OtherActor :type Actor%20Object%20Reference)))

(event EventTick
  (params (DeltaSeconds :type Float%20%28single-precision%29)))

(fn ConstructionScript)

(fn ToggleAlertSprite
  (params (IsVisible :type Boolean))
  (Rendering|SetVisibility (Variables|Default|GetAlert) IsVisible false)
  (Rendering|SetVisibility (Variables|Default|GetAlertDot) IsVisible false))
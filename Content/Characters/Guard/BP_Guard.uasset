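; BP_Guard is a guard character that patrols randomly and chases pawns it spots.
; From BeginPlay, it moves to random navigable points within a radius of its current location, choosing another after each successful move.
; PawnSensing sightings raise walk speed and start an AIMoveTo toward the seen pawn.
; A retriggerable delay, refreshed by each sighting, restores the slower speed and resumes patrol shortly after sightings stop.
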(event OnSeePawn(PawnSensing)
  (params (Pawn :type Pawn%20Object%20Reference))
  ;[0.06125 0.8714 0.2664] On See Player
  (Utilities|FlowControl|Sequence
    (:then_0
      (Variables|/Script/Engine.CharacterMovementComponent|SetMaxWalkSpeed (Variables|Character|GetCharacterMovement) 7e+02))
    (:then_1
      (AI|AIMoveTo self "0, 0, 0" Pawn 5.0 false
        (:then
          (Utilities|FlowControl|RetriggerableDelay 2.0)
          (Variables|/Script/Engine.CharacterMovementComponent|SetMaxWalkSpeed (Variables|Character|GetCharacterMovement) 2.5e+02)
          (CallFunction|RandomPatrol))))))

(event Custom|RandomPatrol
  ;[0.06125 0.8714 0.2664] Patrol Logic
  (bind _randomlocation (Class|NavigationSystemV1|GetRandomLocationinNavigableRadius (Transformation|GetActorLocation) 1e+03 0 0))
  (AI|AIMoveTo self _randomlocation 0 5.0 false
    (:OnSuccess
      (CallFunction|RandomPatrol))))

(event EventBeginPlay
  (CallFunction|RandomPatrol))

(fn ConstructionScript)